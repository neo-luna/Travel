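; Player ship Blueprint that handles the ship's death effects and the switch to the game over screen.
; EndPlay spawns an AsteroidBlast emitter at the ship's location, tinted with primary and secondary colors.
; Destroyed shows the mouse cursor, adds WB_GameOver with game-and-UI input focus, and removes WB_Score.
; Logic toggling two particle systems by movement input is disconnected, and BeginPlay, Tick and overlap events are empty.
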(event `self.ReceiveBeginPlay`)

(event `self.ReceiveTick`
  (params (DeltaSeconds :type "Float (single-precision)")))

(event `self.ReceiveEndPlay`
  (params (EndPlayReason :type "EEndPlayReason Enum" :default "Destroyed"))
  ;[1 1 1 1 60] Particles after destroy
  (`|ExecutionSequence`
    (:`then_0`
      (bind _returnvalue (`GameplayStatics.SpawnEmitterAtLocation` "/Game/PARTICLES/AsteroidBlast.AsteroidBlast" (`self.K2_GetActorLocation`)))
      (`FXSystemComponent.SetColorParameter` _returnvalue "PrimaryColor" (`self.PrimaryColor`))
      (`FXSystemComponent.SetColorParameter` _returnvalue "SecondaryColor" (`self.SecondaryColor`)))))

(event `self.ReceiveDestroyed`
  (bind _returnvalue (`GameplayStatics.GetPlayerController` 0))
  (`|ExecutionSequence`
    (:`then_0`
      ;[1 1 1 1 60] Adding Game Over Menu after PlayerShip destroing
      (set `PlayerController.bShowMouseCursor` true _returnvalue)
      (bind _returnvalue_2 (`|CreateWidget` "/Game/INTERFACE/WB_GameOver.WB_GameOver_C" _returnvalue))
      (bind _output_get (set `self.NewVar_1` _returnvalue_2))
      (`UserWidget.AddToViewport` _output_get 0)
      (`WidgetBlueprintLibrary.SetInputMode_GameAndUIEx` (`GameplayStatics.GetPlayerController` 0) _output_get))
    (:`then_1`
      ;[1 1 1] Remove WB_Score from screen after PlayerShip destroying
      (bind _foundwidgets (`WidgetBlueprintLibrary.GetAllWidgetsOfClass` "/Game/INTERFACE/WB_Score.WB_Score_C"))
      (`Widget.RemoveFromParent` _foundwidgets))))

(fn `UserConstructionScript`)